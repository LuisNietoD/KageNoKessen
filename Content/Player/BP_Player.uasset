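; BP_Player is the player character, with world-axis movement and a vanishing multi-slash attack on nearby enemies through Enhanced Input.
; Attacking hides the mesh and unpauses a looping timer that steps through BP_Enemy actors overlapping its sphere.
; Each step plays a death animation, hides the enemy's head bone and spawns a randomly rotated BP_SlashAttack there.
; A delay scaled by enemy count precedes the player's reappearance.
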(event `EnhancedInput|/Game/Player/Input/IA_Move`
  (params (ActionValue :type "Vector2D Structure") (ElapsedSeconds :type "Float (double-precision)") (TriggeredSeconds :type "Float (double-precision)") (InputAction :type "InputAction Object Reference" :default "/Game/Player/Input/IA_Move.IA_Move"))
  (bind (_x _y) (`KismetMathLibrary.BreakVector2D` ActionValue))
  (:`Triggered`
    (`self.AddMovementInput` (1.0 0.0 0.0) _x true)
    (`self.AddMovementInput` (0.0 1.0 0.0) _y true)))

(event `EnhancedInput|/Game/Player/Input/IA_Attack`
  (params (ActionValue :type Boolean) (ElapsedSeconds :type "Float (double-precision)") (TriggeredSeconds :type "Float (double-precision)") (InputAction :type "InputAction Object Reference" :default "/Game/Player/Input/IA_Attack.IA_Attack"))
  (:`Started`
    (`self.F_HidePlayer` true)
    (set `self.SlashIndex` 0)
    (`KismetSystemLibrary.K2_UnPauseTimer` null "F_Slash")
    (`KismetSystemLibrary.Delay` (+ (* (`KismetArrayLibrary.Array_Length` (`PrimitiveComponent.GetOverlappingActors` (`self.Sphere`) "/Game/BP_Enemy.BP_Enemy_C")) 0.2) 0.2))
    (`SkeletalMeshComponent.PlayAnimation` (`self.Mesh`) "/Game/Player/Models/Animation/Standing.Standing" false)
    (`self.F_HidePlayer` false)))

(event `self.ReceiveBeginPlay`
  (`EnhancedInputSubsystemInterface.AddMappingContext` (pcsubsystem `EnhancedInputLocalPlayerSubsystem` (`GameplayStatics.GetPlayerController` 0)) "/Game/Player/Input/IMC_Inputs.IMC_Inputs" 0 (struct))
  (`KismetSystemLibrary.K2_SetTimer` null "F_Slash" 0.1 true)
  (`KismetSystemLibrary.K2_PauseTimer` null "F_Slash"))

(fn `F_HidePlayer`
  (params (Hide :type Boolean))
  (`SceneComponent.SetHiddenInGame` (`self.Mesh`) Hide false))

(fn `F_Slash`
  (bind _overlappingactors (`PrimitiveComponent.GetOverlappingActors` (`self.Sphere`) "/Game/BP_Enemy.BP_Enemy_C"))
  (bind _output (`|GetArrayItem` _overlappingactors (`self.SlashIndex`)))
  (bind _returnvalue_location (`KismetMathLibrary.BreakTransform` (`self.GetTransform` _output)))
  (if (< (`self.SlashIndex`) (`KismetArrayLibrary.Array_Length` _overlappingactors))
    (bind _asbp_enemy (cast `/Game/BP_Enemy` _output))
    (bind _skeletalmesh (`/Game/BP_Enemy.SkeletalMesh` _asbp_enemy))
    (`SkeletalMeshComponent.PlayAnimation` _skeletalmesh "/Game/Player/Models/Animation/Standing_React_Death_Backward.Standing_React_Death_Backward" false)
    (`SkinnedMeshComponent.HideBoneByName` _skeletalmesh "Head" "PBO_None")
    (`|SpawnActorFromClass` "/Game/BP_SlashAttack.BP_SlashAttack_C" (`KismetMathLibrary.MakeTransform` _returnvalue_location (`KismetMathLibrary.MakeRotator` 0.0 0.0 (`KismetMathLibrary.RandomFloatInRange` 0.0 360.0))) "AlwaysSpawn" "MultiplyWithRoot" null null)
    (`/Engine/EditorBlueprintResources/StandardMacros.IncrementInt` (`self.SlashIndex`)
      (:`  `
        (return)))
    (else
      (`KismetSystemLibrary.K2_PauseTimer` null "F_Slash"))))

(fn `UserConstructionScript`)